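; Manages a Paper2D tile map, spawning gameplay actors from tile user data and copying tiles between maps.
; Setup events store the tile map helper, dimensions and layer count used by both operations.
; Feature spawning scans the target layer for vines, checkpoints (skipped once HasInitializedOnce is set), Goliaths and seeds.
; Copying writes every layer and rebuilds collision; both loops derive Y by dividing by MapHeight, which assumes square maps.
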(event Custom|TrySpawnFeatureActors
  (bind _targettilemaphelper (Variables|Default|GetTargetTileMapHelper))
  (bind _papertilemap (Variables|/Game/Blueprints/TilesetManagement/BP_TileHelper.BP_TileHelper_C|GetPaperTileMap _targettilemaphelper))
  ;[0 1 0.1535] Comment
  (Utilities|IsValid (Variables|Default|GetTargetTileMapHelper) ; Ensure Helper is setup first
    (:Is%20Valid
      ;;[0.05098 0.05098 0.05098] Convert to 1D array
      (for _index (range 0 (- (* (Variables|Default|GetMap%20Width) (Variables|Default|GetMap%20Height)) 0))
        (switch name (Class|TileMapBlueprintLibrary|GetTileUserData (Class|PaperTileMapComponent|GetTile _papertilemap (Math|Integer|%(Integer) _index (Variables|Default|GetMap%20Width)) (/ _index (Variables|Default|GetMap%20Height)) (Variables|Default|GetTargetLayer)))
          (:Default
            (if (not (== (Class|TileMapBlueprintLibrary|GetTileUserData (Class|PaperTileMapComponent|GetTile _papertilemap (Math|Integer|%(Integer) _index (Variables|Default|GetMap%20Width)) (/ _index (Variables|Default|GetMap%20Height)) (Variables|Default|GetTargetLayer))) ""))
              (Development|PrintText (Utilities|Text|FormatText "Attempted to add invalid player feature {name} at {x},{y}" (Class|TileMapBlueprintLibrary|GetTileUserData (Class|PaperTileMapComponent|GetTile _papertilemap (Math|Integer|%(Integer) _index (Variables|Default|GetMap%20Width)) (/ _index (Variables|Default|GetMap%20Height)) (Variables|Default|GetTargetLayer))) (Math|Integer|%(Integer) _index (Variables|Default|GetMap%20Width)) (/ _index (Variables|Default|GetMap%20Height))))))
          (:Vines
            (Game|SpawnActorfromClass "/Game/Blueprints/TilesetManagement/BP_ClimableTilette.BP_ClimableTilette_C" (Math|Transform|MakeTransform (Math|Vector|MakeVector (.x (Class|PaperTileMapComponent|GetTileCenterPosition _papertilemap (Math|Integer|%(Integer) _index (Variables|Default|GetMap%20Width)) (/ _index (Variables|Default|GetMap%20Height)) (Variables|Default|GetTargetLayer) true)) (.y (Class|PaperTileMapComponent|GetTileCenterPosition _papertilemap (Math|Integer|%(Integer) _index (Variables|Default|GetMap%20Width)) (/ _index (Variables|Default|GetMap%20Height)) (Variables|Default|GetTargetLayer) true)) (.z (Class|PaperTileMapComponent|GetTileCenterPosition _papertilemap (Math|Integer|%(Integer) _index (Variables|Default|GetMap%20Width)) (/ _index (Variables|Default|GetMap%20Height)) (Variables|Default|GetTargetLayer) true))) "0, 0, 0" "1.000000,1.000000,1.000000") "AlwaysSpawn" 0 0)
            (Development|PrintText (Utilities|Text|FormatText "Spawned climbable tile at {x},{y}" (Math|Integer|%(Integer) _index (Variables|Default|GetMap%20Width)) (/ _index (Variables|Default|GetMap%20Height)))))
          (:Checkpoint
            (if (not (Variables|Default|GetHasInitializedOnce))
              (Game|SpawnActorfromClass "/Game/Blueprints/BP_SpriteCheckpoint.BP_SpriteCheckpoint_C" (Math|Transform|MakeTransform (Math|Vector|MakeVector (.x (Class|PaperTileMapComponent|GetTileCenterPosition _papertilemap (Math|Integer|%(Integer) _index (Variables|Default|GetMap%20Width)) (/ _index (Variables|Default|GetMap%20Height)) (Variables|Default|GetTargetLayer) true)) (.y (Class|PaperTileMapComponent|GetTileCenterPosition _papertilemap (Math|Integer|%(Integer) _index (Variables|Default|GetMap%20Width)) (/ _index (Variables|Default|GetMap%20Height)) (Variables|Default|GetTargetLayer) true)) (.z (Class|PaperTileMapComponent|GetTileCenterPosition _papertilemap (Math|Integer|%(Integer) _index (Variables|Default|GetMap%20Width)) (/ _index (Variables|Default|GetMap%20Height)) (Variables|Default|GetTargetLayer) true))) "0, 0, 0" "1.000000,1.000000,1.000000") "AlwaysSpawn" 0 0)
              (Development|PrintText (Utilities|Text|FormatText "Spawned checkpoint tile at {x},{y}" (Math|Integer|%(Integer) _index (Variables|Default|GetMap%20Width)) (/ _index (Variables|Default|GetMap%20Height))))))
          (:Goliath
            (Game|SpawnActorfromClass "/Game/Blueprints/BP_SpriteGoliath.BP_SpriteGoliath_C" (Math|Transform|MakeTransform (Math|Vector|MakeVector (.x (Class|PaperTileMapComponent|GetTileCenterPosition _papertilemap (Math|Integer|%(Integer) _index (Variables|Default|GetMap%20Width)) (/ _index (Variables|Default|GetMap%20Height)) (Variables|Default|GetTargetLayer) true)) (.y (Class|PaperTileMapComponent|GetTileCenterPosition _papertilemap (Math|Integer|%(Integer) _index (Variables|Default|GetMap%20Width)) (/ _index (Variables|Default|GetMap%20Height)) (Variables|Default|GetTargetLayer) true)) (.z (Class|PaperTileMapComponent|GetTileCenterPosition _papertilemap (Math|Integer|%(Integer) _index (Variables|Default|GetMap%20Width)) (/ _index (Variables|Default|GetMap%20Height)) (Variables|Default|GetTargetLayer) true))) "0, 0, 0" "1.000000,1.000000,1.000000") "AlwaysSpawn" 0 0)
            (Development|PrintText (Utilities|Text|FormatText "Spawned Goliath at {x},{y}" (Math|Integer|%(Integer) _index (Variables|Default|GetMap%20Width)) (/ _index (Variables|Default|GetMap%20Height)))))
          (:Seed
            (Game|SpawnActorfromClass "/Game/Blueprints/BP_SpriteSeed.BP_SpriteSeed_C" (Math|Transform|MakeTransform (Math|Vector|MakeVector (.x (Class|PaperTileMapComponent|GetTileCenterPosition _papertilemap (Math|Integer|%(Integer) _index (Variables|Default|GetMap%20Width)) (/ _index (Variables|Default|GetMap%20Height)) (Variables|Default|GetTargetLayer) true)) (.y (Class|PaperTileMapComponent|GetTileCenterPosition _papertilemap (Math|Integer|%(Integer) _index (Variables|Default|GetMap%20Width)) (/ _index (Variables|Default|GetMap%20Height)) (Variables|Default|GetTargetLayer) true)) (.z (Class|PaperTileMapComponent|GetTileCenterPosition _papertilemap (Math|Integer|%(Integer) _index (Variables|Default|GetMap%20Width)) (/ _index (Variables|Default|GetMap%20Height)) (Variables|Default|GetTargetLayer) true))) "0, 0, 0" "1.000000,1.000000,1.000000") "Undefined" 0 0)
            (Development|PrintText (Utilities|Text|FormatText "Spawned Seed at {x},{y}" (Math|Integer|%(Integer) _index (Variables|Default|GetMap%20Width)) (/ _index (Variables|Default|GetMap%20Height))))))))))

(event Custom|ConfigureMapProperties
  (params (TargetMap :type Paper%20Tile%20Map%20Object%20Reference))
  ;[1 0 0.8784] Comment
  (Variables|Default|SetMap%20Width (Variables|/Script/Paper2D.PaperTileMap|GetMapWidth TargetMap))
  (Variables|Default|SetMap%20Height (Variables|/Script/Paper2D.PaperTileMap|GetMapHeight TargetMap))
  (Variables|Default|SetMap%20Total%20Layer%20Depth (Utilities|Array|Length (Variables|/Script/Paper2D.PaperTileMap|GetTileLayers TargetMap))))

(event Custom|CopyTileMap
  (params (To :type Paper%20Tile%20Map%20Component%20Object%20Reference) (From :type Paper%20Tile%20Map%20Actor%20Object%20Reference))
  ;[1 0.2457 0] Copy TileMap
  (Utilities|IsValid (Variables|Default|GetTargetTileMapHelper) ; Ensure Helper is setup first
    (:Is%20Valid
      (if (> (Variables|Default|GetMap%20Total%20Layer%20Depth) 0) ; Must have atleast one layer to copy
        (for _index (range 0 (- (Variables|Default|GetMap%20Total%20Layer%20Depth) 1)) ; For Each Layer
          (Class|PaperTileMapComponent|RebuildCollision To)
          (Development|PrintText (Utilities|Text|FormatText "Layer {layer}" _index) true true "(R=1.000000,G=0.000000,B=0.570890,A=1.000000)")
          (for _index_2 (range 0 (- (* (Variables|Default|GetMap%20Width) (Variables|Default|GetMap%20Height)) 0)) ; For each Tile
            (Development|PrintText (Utilities|Text|FormatText "Tile Id {id}" (.TileIndex (Class|TileMapBlueprintLibrary|BreakTile (Class|PaperTileMapComponent|GetTile (Variables|/Script/Paper2D.PaperTileMapActor|GetRenderComponent From) (Math|Integer|%(Integer) _index_2 (Variables|Default|GetMap%20Width)) (/ _index_2 (Variables|Default|GetMap%20Height)) _index)))) true true "(R=1.000000,G=0.000000,B=0.570890,A=1.000000)")
            (Class|PaperTileMapComponent|SetTile To (Math|Integer|%(Integer) _index_2 (Variables|Default|GetMap%20Width)) (/ _index_2 (Variables|Default|GetMap%20Height)) _index (Class|PaperTileMapComponent|GetTile (Variables|/Script/Paper2D.PaperTileMapActor|GetRenderComponent From) (Math|Integer|%(Integer) _index_2 (Variables|Default|GetMap%20Width)) (/ _index_2 (Variables|Default|GetMap%20Height)) _index))))
        (Class|PaperTileMapComponent|RebuildCollision To)
        (Development|PrintText "COPY TILE COMPLETE" true true "(R=0.000000,G=1.000000,B=0.000000,A=1.000000)")))))

(event Custom|ConfigureTileMapHelperRef
  (params (Tile%20Helper :type BP%20Tile%20Helper%20Object%20Reference))
  ;[1 0 0.8784] Comment
  (Variables|Default|SetTargetTileMapHelper Tile%20Helper))

(event EventBeginPlay
  ;[1 0 0.8784] Comment
)

(event Collision|EventActorBeginOverlap
  (params (OtherActor :type Actor%20Object%20Reference)))

(event EventTick
  (params (DeltaSeconds :type Float%20%28single-precision%29)))

(fn ConstructionScript)