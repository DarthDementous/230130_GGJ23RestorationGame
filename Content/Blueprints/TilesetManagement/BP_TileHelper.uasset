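; BP_TileHelper is an actor that owns a runtime-created Paper2D tilemap and allows its tiles to be changed during play.
; On BeginPlay it registers with the player's BP_SpriteCharacter and can replicate an existing map's layers.
; BP_TilesetManager handles map configuration, tile copying and feature actor spawning for that copy.
; ChangeTile sets a tile by position, layer and tileset, then rebuilds collision.
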(event Custom|ChangeTile
  (params (Grid%20Pos%20X :type Integer) (Grid%20Pos%20Y :type Integer) (Grid%20Layer%20Id :type Integer) (Source%20Tile%20Id :type Integer) (Source%20Tile%20Set :type Paper%20Tile%20Set%20Object%20Reference))
  (bind _papertilemap (Variables|Default|GetPaperTileMap))
  (Class|PaperTileMapComponent|SetTile _papertilemap Grid%20Pos%20X Grid%20Pos%20Y Grid%20Layer%20Id (Class|TileMapBlueprintLibrary|MakeTile Source%20Tile%20Id Source%20Tile%20Set))
  (Class|PaperTileMapComponent|RebuildCollision _papertilemap)
  (Development|PrintText (Utilities|Text|FormatText "Changed tile at {x},{y}" Grid%20Pos%20X Grid%20Pos%20Y)))

(event Collision|EventActorBeginOverlap
  (params (OtherActor :type Actor%20Object%20Reference)))

(event EventTick
  (params (DeltaSeconds :type Float%20%28single-precision%29)))

(event EventBeginPlay
  (bind _papertilemap (Variables|Default|GetPaperTileMap))
  (Class|PaperTileMapComponent|CreateNewTileMap _papertilemap (Variables|TileMapCreation|GetMap%20Width) (Variables|TileMapCreation|GetMap%20Height) (Variables|TileMapCreation|GetTile%20Width) (Variables|TileMapCreation|GetTile%20Height) (Variables|TileMapCreation|GetPixels%20Per%20Unreal%20Unit) (Variables|TileMapCreation|GetCreate%20Empty%20Layer))
  (if (Class|PaperTileMapComponent|OwnsTileMap _papertilemap)
    (Utilities|FlowControl|Sequence
      (:then_0
        (Utilities|IsValid (Variables|Default|GetTileSetManager) ; Incase we forgot to assign in scene, try and find the first occurance
          (:Is%20Valid
            (bind _returnvalue (Actor|GetActorOfClass "/Game/Blueprints/TilesetManagement/BP_TilesetManager.BP_TilesetManager_C"))
            (Variables|Default|SetTileSetManager _returnvalue))))
      (:then_1
        (bind _asbp_sprite_character (Utilities|Casting|CastToBP_SpriteCharacter (Game|GetPlayerCharacter 0)))
        (Variables|/Game/Blueprints/BP_SpriteCharacter.BP_SpriteCharacter_C|SetTile%20Helper _asbp_sprite_character self))
      (:then_2
        (if (Variables|Default|GetShouldPropogateExistingMap)
          (if (and (Utilities|IsValid (Variables|Default|GetExisitingTileMap)) (Utilities|IsValid (Variables|Default|GetTileSetManager)))
            (Variables|TileMapCreation|SetMap%20Depth (Utilities|Array|Length (Variables|/Script/Paper2D.PaperTileMap|GetTileLayers (Variables|/Script/Paper2D.PaperTileMapComponent|GetTileMap (Variables|/Script/Paper2D.PaperTileMapActor|GetRenderComponent (Variables|Default|GetExisitingTileMap))))))
            (for _index (range 0 (- (Variables|TileMapCreation|GetMap%20Depth) 1)) ; Ensure our created map has the same number of layers as the input map
              (if (< (Utilities|Array|Length (Variables|/Script/Paper2D.PaperTileMap|GetTileLayers (Variables|/Script/Paper2D.PaperTileMapComponent|GetTileMap (Variables|Default|GetPaperTileMap)))) (Variables|TileMapCreation|GetMap%20Depth))
                (Class|PaperTileMapComponent|AddNewLayer (Variables|Default|GetPaperTileMap))))
            ;[1 0.4246 0.04267] Setup map copy and spawning
            (Default|ConfigureTileMapHelperRef (Variables|Default|GetTileSetManager) self)
            (Default|ConfigureMapProperties (Variables|Default|GetTileSetManager) (Variables|/Script/Paper2D.PaperTileMapComponent|GetTileMap (Variables|/Script/Paper2D.PaperTileMapActor|GetRenderComponent (Variables|Default|GetExisitingTileMap)))) ; Use properties of existiing map for initial setup
            (Default|CopyTileMap (Variables|Default|GetTileSetManager) (Variables|Default|GetPaperTileMap) (Variables|Default|GetExisitingTileMap))
            (Default|ConfigureMapProperties (Variables|Default|GetTileSetManager) (Variables|/Script/Paper2D.PaperTileMapComponent|GetTileMap (Variables|Default|GetPaperTileMap)))
            (Default|TrySpawnFeatureActors (Variables|Default|GetTileSetManager))))))))

(fn ConstructionScript)