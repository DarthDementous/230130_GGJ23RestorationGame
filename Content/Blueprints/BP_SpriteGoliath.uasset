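; BP_SpriteGoliath is a character that patrols back and forth automatically, starting along positive X.
; Each Tick it applies movement along CurrDir and runs two debug-drawn line traces: forward-down for ledges, short forward for walls.
; A missing floor or a wall hit calls SwapDirections, which negates CurrDir and sets a one-second cooldown against repeated flips.
; The capsule hit event is empty, leaving its direction-swap logic disconnected.
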(event OnComponentHit(CapsuleComponent)
  (params (HitComponent :type Primitive%20Component%20Object%20Reference) (OtherActor :type Actor%20Object%20Reference) (OtherComp :type Primitive%20Component%20Object%20Reference) (NormalImpulse :type Vector :default "0, 0, 0") (Hit :type Hit%20Result%20Structure%20%28by%20ref%29)))

(event Custom|SwapDirections
  (Variables|Default|SetCurrDir (Class|KismetMathLibrary|Negated2D (Variables|Default|GetCurrDir)))
  (Variables|Default|SetHasSwappedDir true)
  ;[0.05098 0.05098 0.05098] Wait a bit so we don't immediately swap directions again
  (Utilities|FlowControl|Delay 1.0)
  (Variables|Default|SetHasSwappedDir false))

(event EventBeginPlay
  ;[0.05098 0.05098 0.05098] Start by moving right
  (Variables|Default|SetCurrDir "(X=1.000000,Y=0.000000)"))

(event EventTick
  (params (DeltaSeconds :type Float%20%28single-precision%29))
  (bind _returnvalue (Transformation|GetActorLocation))
  (bind _returnvalue_2 (Transformation|GetActorLocation))
  ;[0.05098 0.05098 0.05098] Walk in current direction
  (Pawn|Input|AddMovementInput (Math|Conversions|ToVector(Vector2D) (Variables|Default|GetCurrDir)) 1.0 false)
  (Utilities|FlowControl|Sequence
    (:then_0
      ;[0.05098 0.05098 0.05098] About to fall, swap directions (if not doing so already)
      (bind _returnvalue_3 (Collision|LineTraceByChannel _returnvalue (+ _returnvalue (+ (* (Transformation|GetActorForwardVector) 8e+01) "0.000000,0.000000,-80.000000")) "TraceTypeQuery1" false 0 "ForDuration" true "(R=1.000000,G=0.000000,B=0.000000,A=1.000000)" "(R=0.000000,G=1.000000,B=0.000000,A=1.000000)" 0.25))
      (if (not _returnvalue_3)
        (if (not (Variables|Default|GetHasSwappedDir))
          (CallFunction|SwapDirections))))
    (:then_1
      (bind (_outhit _returnvalue_4) (Collision|LineTraceByChannel _returnvalue_2 (+ _returnvalue_2 (+ (* (Transformation|GetActorForwardVector) 3e+01) (Math|Vector|MakeVector -5.0 1e+01 0.0))) "TraceTypeQuery1" false 0 "ForDuration" true "(R=1.000000,G=0.000000,B=0.000000,A=1.000000)" "(R=0.000000,G=1.000000,B=0.000000,A=1.000000)" 0.25))
      (if _returnvalue_4
        (if (not (Variables|Default|GetHasSwappedDir))
          (CallFunction|SwapDirections))))))

(fn ConstructionScript)