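; BP_SpriteCheckpoint is a sprite-based checkpoint that activates on actor overlap.
; It requires the "Interaction" tag on the first component in the other actor's overlapping-components list, then swaps to the activated sprite.
; It adds itself uniquely to BP_TilesetManager's CheckpointArray and writes the returned index to the controlled BP_SpriteCharacter's LastCheckpointIndex, printing a confirmation.
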(event Collision|EventActorBeginOverlap
  (params (OtherActor :type Actor%20Object%20Reference))
  (bind _output_get (Variables|Default|SetIsActivated (Utilities|Array|ContainsItem (Variables|/Script/Engine.ActorComponent|GetComponentTags (Utilities|Array|Get(acopy) (Class|Actor|GetOverlappingComponents OtherActor))) "Interaction")))
  (if _output_get
    ;[0.05098 0.05098 0.05098] Change to activated sprite
    (Rendering|Components|Sprite|SetSprite (Variables|Default|GetRenderComponent) "/Game/Tilesets/spirit_bulb_collision.spirit_bulb_collision")
    (bind _asbp_sprite_character (Utilities|Casting|CastToBP_SpriteCharacter (Pawn|GetControlledPawn (Game|GetPlayerController 0))))
    (bind _returnvalue (Actor|GetActorOfClass "/Game/Blueprints/TilesetManagement/BP_TilesetManager.BP_TilesetManager_C"))
    ;[0.05098 0.05098 0.05098] Add activated checkpoint to array and update on player
    (bind _returnvalue_2 (Utilities|Array|AddUnique (Variables|/Game/Blueprints/TilesetManagement/BP_TilesetManager.BP_TilesetManager_C|GetCheckpointArray _returnvalue) self))
    (bind _output_get_2 (Variables|Default|SetCheckpointIndex _returnvalue_2))
    (Variables|/Game/Blueprints/BP_SpriteCharacter.BP_SpriteCharacter_C|SetLastCheckpointIndex _asbp_sprite_character _output_get_2)
    (Development|PrintText (Utilities|Text|FormatText "Activated checkpoint {index}" _output_get_2))))

(fn ConstructionScript)