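; Player character for a 2D Paper2D platformer, with Enhanced Input side-scrolling movement, jumping, and a howl interaction that also converts the tile at its position as a test.
; Tick picks movement flipbooks from velocity, while CheckCanPlayNewAnim protects one-shot Land, Howl and Collapse animations.
; "Kill" overlaps trigger death, which freezes input and gravity, then after a delay destroys DynamicEntity actors, resets the tilemap and respawns at the last checkpoint or PlayerStart.
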(event OnFinishedPlaying(Sprite)
  (if (or (Utilities|Enum|Equal(Enum) (Variables|Default|GetLastPlayedAnim) "Land") (Utilities|Enum|Equal(Enum) (Variables|Default|GetLastPlayedAnim) "Howl"))
    (Variables|Default|SetLastPlayedAnim "Idle")
    (Sprite|SetFlipbook (Variables|Default|GetSprite) "/Game/Sprites/Characters/Spirit/Idle/player-movement-idle.player-movement-idle")
    (CallFunction|RestartFlipbook :!label _label)
    (elif (Utilities|Enum|Equal(Enum) (Variables|Default|GetLastPlayedAnim) "Collapse")
      (Variables|Default|SetLastPlayedAnim "Idle")
      (Sprite|SetFlipbook (Variables|Default|GetSprite) "/Game/Sprites/Characters/Spirit/Idle/player-movement-idle.player-movement-idle")
      (goto _label))))

(event OnComponentBeginOverlap(CapsuleComponent)
  (params (OverlappedComponent :type Primitive%20Component%20Object%20Reference) (OtherActor :type Actor%20Object%20Reference) (OtherComp :type Primitive%20Component%20Object%20Reference) (OtherBodyIndex :type Integer) (bFromSweep :type Boolean) (SweepResult :type Hit%20Result%20Structure%20%28by%20ref%29))
  ;[0.05098 0.05098 0.05098] Killed by hurtbox (and not already dead)
  (if (Utilities|Array|ContainsItem (Variables|/Script/Engine.ActorComponent|GetComponentTags OtherComp) "Kill")
    (if (not (Variables|Default|GetIsDead))
      (Utilities|FlowControl|Sequence
        (:then_0
          (CallFunction|OnDeath))
        (:then_1
          (bind _asbp_sprite_goliath (Utilities|Casting|CastToBP_SpriteGoliath OtherActor))
          (Default|OnAttack _asbp_sprite_goliath))))))

(event Custom|OnInteract
  (bind _sprite (Variables|Default|GetSprite))
  ;[1 1 1] Debug Actions via input
  (Components|Timeline|SetLooping _sprite false) ; Special Feature animations for sprite do not loop and 'play once'.
  (Variables|Default|SetLastPlayedAnim "Howl")
  (Sprite|SetFlipbook _sprite "/Game/Sprites/Characters/Spirit/Howl/player-movement-howl.player-movement-howl"))

(event Custom|OnBeginRestart
  (bind _sprite (Variables|Default|GetSprite))
  ;[1 1 1] Debug Actions via input
  (Components|Timeline|SetLooping _sprite false) ; Special Feature animations for sprite do not loop and 'play once'.
  (Variables|Default|SetLastPlayedAnim "Collapse")
  (Sprite|SetFlipbook _sprite "/Game/Sprites/Characters/Spirit/Collapse/player-movement-export-collapse.player-movement-export-collapse"))

(event Custom|UpdateAnimation
  (bind _returnvalue (Pawn|GetController))
  (bind _charactermovement (Variables|Character|GetCharacterMovement))
  (bind _charactermovement_2 (Variables|Character|GetCharacterMovement))
  (bind _runspeedthreshold (Variables|Default|GetRunSpeedThreshold))
  (bind _returnvalue_2 (AI|Components|NavMovement|IsFalling _charactermovement))
  (bind _velocity (Variables|/Script/Engine.MovementComponent|GetVelocity _charactermovement_2))
  (bind _returnvalue_3 (Math|Vector|VectorLength _velocity))
  (bind (_x _y _z) (Math|Vector|BreakVector _velocity))
  (bind _returnvalue_4 (Math|Float|Absolute(Float) _x))
  (bind _returnvalue_5 (== _z 0.0))
  (bind _returnvalue_6 (> _returnvalue_3 0.0))
  (bind _returnvalue_7 (> _z 0.0))
  (bind _returnvalue_8 (> _returnvalue_4 _runspeedthreshold))
  (bind _canplay (CallFunction|CheckCanPlayNewAnim false))
  ;[0.05098 0.05098 0.05098] Movement animation
  (if _canplay
    (bind _output_get (Variables|Default|SetLastPlayedAnim (select _returnvalue_2 (select _returnvalue_7 "Jump" (select _returnvalue_5 "Hover" "Fall")) (select _returnvalue_6 (select _returnvalue_8 "Leap" "Walk") "Idle"))))
    (switch string _output_get
      (:Idle
        _)
      (:Walk
        _)
      (:Leap
        _)
      (:Hover
        _)
      (:Fall
        _)
      (:Collapse
        _)
      (:Howl
        _)
      (:Land
        _)
      (:Jump
        _))
    (Sprite|SetFlipbook (Variables|Default|GetSprite) (select _returnvalue_2 (select _returnvalue_7 "/Game/Sprites/Characters/Spirit/Jump/player-movement-jump.player-movement-jump" (select _returnvalue_5 "/Game/Sprites/Characters/Spirit/Hover/player-movement-hover.player-movement-hover" "/Game/Sprites/Characters/Spirit/Fall/player-movement-fall.player-movement-fall")) (select _returnvalue_6 (select _returnvalue_8 "/Game/Sprites/Characters/Spirit/Leap/player-movement-leap.player-movement-leap" "/Game/Sprites/Characters/Spirit/Walk/player-movement-walk.player-movement-walk") "/Game/Sprites/Characters/Spirit/Idle/player-movement-idle.player-movement-idle")))
    (CallFunction|RestartFlipbook)
    (Math|Float|CompareFloat _x 0.0
      (:>
        (Pawn|SetControlRotation _returnvalue (Math|Rotator|MakeRotator 0.0 0.0 1.8e+02)))
      (:<
        (Pawn|SetControlRotation _returnvalue (Math|Rotator|MakeRotator 0.0 0.0 0.0))))))

(event Custom|OnDeath
  (bind _charactermovement (Variables|Character|GetCharacterMovement))
  ;[0.05098 0.05098 0.05098] Death
  (Variables|Default|SetIsDead true)
  (Class|EnhancedInputSubsystemInterface|ClearAllMappings (PlayerController|LocalPlayerSubsystems|GetEnhancedInputLocalPlayerSubsystem (Game|GetPlayerController 0)))
  ;[1 1 1] Hooked to Death Anim
  (CallFunction|OnBeginRestart)
  (Components|Movement|StopMovementImmediately _charactermovement)
  (Variables|/Script/Engine.CharacterMovementComponent|SetGravityScale _charactermovement 0.0)
  (Utilities|FlowControl|Delay 2.0)
  (CallFunction|OnRespawn))

(event Custom|OnRespawn
  ;[0.05098 0.05098 0.05098] Respawn
  (Variables|Default|SetIsDead false)
  ;[0.05098 0.05098 0.05098] Respawn the entities (except for static ones)
  (bind _outactors (Actor|GetAllActorswithTag "DynamicEntity"))
  (for _array_element _outactors
    (Actor|DestroyActor _array_element))
  ;[0.05098 0.05098 0.05098] Reset the map
  (Default|SetupMap (Variables|Default|GetTile%20Helper))
  (Input|AddMappingContext (PlayerController|LocalPlayerSubsystems|GetEnhancedInputLocalPlayerSubsystem (Game|GetPlayerController 0)) "/Game/Input/IMC_Default.IMC_Default" 0 "(bIgnoreAllPressedKeysUntilRelease=True,bForceImmediately=False)")
  (Variables|/Script/Engine.CharacterMovementComponent|SetGravityScale (Variables|Character|GetCharacterMovement) (Variables|Default|GetInitialGravityScale))
  (bind _returnvalue (Actor|GetActorOfClass "/Game/Blueprints/TilesetManagement/BP_TilesetManager.BP_TilesetManager_C"))
  (Utilities|IsValid (Utilities|Array|Get(acopy) (Variables|/Game/Blueprints/TilesetManagement/BP_TilesetManager.BP_TilesetManager_C|GetCheckpointArray _returnvalue) (Variables|Default|GetLastCheckpointIndex))
    (:Is%20Valid
      (Transformation|SetActorLocation (Transformation|GetActorLocation (Utilities|Array|Get(acopy) (Variables|/Game/Blueprints/TilesetManagement/BP_TilesetManager.BP_TilesetManager_C|GetCheckpointArray _returnvalue) (Variables|Default|GetLastCheckpointIndex))) false false))
    (:Is%20Not%20Valid
      ;[0.05098 0.05098 0.05098] No checkpoints activated, start at beginning
      (bind _returnvalue_2 (Actor|GetActorOfClass "/Script/Engine.PlayerStart"))
      (Transformation|SetActorLocation (Transformation|GetActorLocation _returnvalue_2) false false)
      (CallFunction|OnForceRespawn))))

(event Custom|RestartFlipbook
  (bind _sprite (Variables|Default|GetSprite))
  ;[1 1 1] Restart Flipbook to animations play smoothly
  (Components|Timeline|SetLooping _sprite true) ; Default animations should loop, unless set within this code to play once
  (Audio|Components|Audio|Play _sprite) ; If the flipbook was set looping as false, a manaul restart is required.
)

(event Custom|OnForceRespawn
  (Variables|Default|SetLastPlayedAnim "Idle")
  (Sprite|SetFlipbook (Variables|Default|GetSprite) "/Game/Sprites/Characters/Spirit/Idle/player-movement-idle.player-movement-idle")
  (CallFunction|RestartFlipbook))

(event Custom|OnChangeTile
  (Default|ConvertExistingTileatWorldPos (Variables|Default|GetTile%20Helper) 2 (Variables|Default|GetConversion%20Tileset) (Transformation|GetWorldLocation (Variables|Collision|GetCapsuleComponent))))

(event Input|EnhancedActionEvents|EnhancedInputActionIA_Respawn
  (params (ActionValue :type Boolean) (ElapsedSeconds :type Float%20%28double-precision%29) (TriggeredSeconds :type Float%20%28double-precision%29) (InputAction :type Input%20Action%20Object%20Reference :default "/Game/Input/IA_Respawn.IA_Respawn"))
  ;[0 1 0.06846] Input
  (:Triggered
    (CallFunction|OnDeath)))

(event Input|EnhancedActionEvents|EnhancedInputActionIA_Interact
  (params (ActionValue :type Boolean) (ElapsedSeconds :type Float%20%28double-precision%29) (TriggeredSeconds :type Float%20%28double-precision%29) (InputAction :type Input%20Action%20Object%20Reference :default "/Game/Input/IA_Interact.IA_Interact"))
  ;[0 1 0.06846] Input
  (:Triggered
    (CallFunction|CheckCanPlayNewAnim true)
    (CallFunction|OnInteract))
  (:Started
    ;;[1 1 1] TESTING
    (CallFunction|OnChangeTile)))

(event Input|EnhancedActionEvents|EnhancedInputActionIA_Move
  (params (ActionValue :type Vector%202D%20Structure) (ElapsedSeconds :type Float%20%28double-precision%29) (TriggeredSeconds :type Float%20%28double-precision%29) (InputAction :type Input%20Action%20Object%20Reference :default "/Game/Input/IA_Move.IA_Move"))
  ;[0 1 0.06846] Input
  (:Triggered
    (bind _canplay (CallFunction|CheckCanPlayNewAnim true))
    (if _canplay
      (Pawn|Input|AddMovementInput "1.000000,0.000000,0.000000" (.x ActionValue) false))))

(event Input|EnhancedActionEvents|EnhancedInputActionIA_Jump
  (params (ActionValue :type Boolean) (ElapsedSeconds :type Float%20%28double-precision%29) (TriggeredSeconds :type Float%20%28double-precision%29) (InputAction :type Input%20Action%20Object%20Reference :default "/Game/Input/IA_Jump.IA_Jump"))
  ;[0 1 0.06846] Input
  (:Triggered
    (bind _canplay (CallFunction|CheckCanPlayNewAnim true))
    (if _canplay
      (Character|Jump)))
  (:Completed
    (Character|StopJumping)))

(event EventOnLanded
  (params (Hit :type Hit%20Result%20Structure%20%28by%20ref%29))
  (bind _sprite (Variables|Default|GetSprite))
  ;[1 1 1] Reactions to player movement
  (Components|Timeline|SetLooping _sprite false) ; Special Feature animations for sprite do not loop and 'play once'.
  (Variables|Default|SetLastPlayedAnim "Land")
  (Sprite|SetFlipbook _sprite "/Game/Sprites/Characters/Spirit/Land/player-movement-land.player-movement-land"))

(event EventBeginPlay
  (bind _outactors (Actor|GetAllActorsOfClass "/Script/Paper2D.PaperTileMapActor"))
  (for _array_element _outactors
    _)
  ;[0.05098 0.05098 0.05098] Initialise input mapping context
  (bind _asplayer_controller (Utilities|Casting|CastToPlayerController (Pawn|GetController)))
  (Utilities|IsValid (PlayerController|LocalPlayerSubsystems|GetEnhancedInputLocalPlayerSubsystem _asplayer_controller)
    (:Is%20Valid
      (Input|AddMappingContext (PlayerController|LocalPlayerSubsystems|GetEnhancedInputLocalPlayerSubsystem _asplayer_controller) "/Game/Input/IMC_Default.IMC_Default" 0 "(bIgnoreAllPressedKeysUntilRelease=True,bForceImmediately=False)"))))

(event EventTick
  (params (DeltaSeconds :type Float%20%28single-precision%29))
  ;[1 1 1] EventTick
  (CallFunction|UpdateAnimation))

(fn ConstructionScript
  (Variables|Default|SetJumpMaxHoldTime (Variables|Default|GetMaxJumpHoldTime))
  (Variables|Default|SetInitialGravityScale (Variables|/Script/Engine.CharacterMovementComponent|GetGravityScale (Variables|Character|GetCharacterMovement))))

(fn CheckCanPlayNewAnim
  (params (Alllow%20Interrupts :type Boolean))
  (bind _lastplayedanim (Variables|Default|GetLastPlayedAnim))
  (bind _returnvalue (Utilities|Enum|NotEqual(Enum) _lastplayedanim "Howl"))
  (bind _returnvalue_2 (Utilities|Enum|NotEqual(Enum) _lastplayedanim "Collapse"))
  (bind _returnvalue_3 (and _returnvalue_2 _returnvalue))
  (return (select Alllow%20Interrupts _returnvalue_3 (and (Utilities|Enum|NotEqual(Enum) (Variables|Default|GetLastPlayedAnim) "Land") _returnvalue_3))))